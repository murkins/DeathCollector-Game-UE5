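; BP_Scroll is a collectible scroll pickup that the player collects by touching it.
; On BeginPlay, the ScrollMovement timeline starts animating the Scroll component's relative height.
; When an actor tagged Player overlaps the Sphere, it gets a game mode reference through a message call, sends AddScrollMessage to it, plays a loot sound and destroys itself.
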(event `self.ReceiveBeginPlay`
  (bind (_direction _locationalpha) (`Timeline|ScrollMovement` :!via `PlayFromStart`)
    (:`Update`
      (`SceneComponent.K2_SetRelativeLocation` (`self.Scroll`) (`KismetMathLibrary.MakeVector` 0.0 0.0 (.z _locationalpha)) false false))))

(event `self.Sphere.OnComponentBeginOverlap`
  (params (OverlappedComponent :type "PrimitiveComponent Object Reference") (OtherActor :type "Actor Object Reference") (OtherComp :type "PrimitiveComponent Object Reference") (OtherBodyIndex :type Integer) (bFromSweep :type Boolean) (SweepResult :type "HitResult Structure (by ref)"))
  (if (`self.ActorHasTag` OtherActor "Player")
    (bind _gamemode (message `/Game/Blueprints/Interfaces/INT_GameMode.SetGameModeRef` (`GameplayStatics.GetGameMode`)))
    (message `/Game/Blueprints/Interfaces/INT_GameMode.AddScroll` _gamemode)
    (`GameplayStatics.PlaySound2D` "/Game/Audio/SFX/SC_Loot.SC_Loot" 1.0 1.0 0.0 null null)
    (`self.K2_DestroyActor`)))

(fn `UserConstructionScript`)