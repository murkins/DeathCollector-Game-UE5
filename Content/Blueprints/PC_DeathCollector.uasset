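; PC_DeathCollector is a controller Blueprint that rolls the player's ball from movement axis input.
; MoveForward and MoveRight get the ball reference from player pawn 0 through a SetBallRefMessage call.
; Each scales its axis value into torque on the ball, around Y for forward and X for right.
; If the pawn is invalid, each handler retries after a short delay.
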(event `InputAxis|MoveForward`
  (params (AxisValue :type "Float (single-precision)"))
  (bind _returnvalue (`GameplayStatics.GetPlayerPawn` 0))
  (`/Engine/EditorBlueprintResources/StandardMacros.IsValid` _returnvalue :!label _label
    (:`Is Valid`
      (bind _ball (message `/Game/Blueprints/Interfaces/INT_Ball.SetBallRef` _returnvalue))
      (`PrimitiveComponent.AddTorqueInRadians` (`/Game/Blueprints/BP_Ball.Ball` _ball) (`KismetMathLibrary.MakeVector` 0.0 (* AxisValue 1000000.0)) "None" false))
    (:`Is Not Valid`
      (`KismetSystemLibrary.Delay` 0.2)
      (goto _label))))

(event `InputAxis|MoveRight`
  (params (AxisValue :type "Float (single-precision)"))
  (bind _returnvalue (`GameplayStatics.GetPlayerPawn` 0))
  (`/Engine/EditorBlueprintResources/StandardMacros.IsValid` _returnvalue :!label _label_2
    (:`Is Valid`
      (bind _ball (message `/Game/Blueprints/Interfaces/INT_Ball.SetBallRef` _returnvalue))
      (`PrimitiveComponent.AddTorqueInRadians` (`/Game/Blueprints/BP_Ball.Ball` _ball) (`KismetMathLibrary.MakeVector` (* AxisValue 1000000.0)) "None" false))
    (:`Is Not Valid`
      (`KismetSystemLibrary.Delay` 0.2)
      (goto _label_2))))

(fn `UserConstructionScript`)