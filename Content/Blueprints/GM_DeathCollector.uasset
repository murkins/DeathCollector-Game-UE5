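; Game mode for DeathCollector that counts looted scrolls and awards a trophy tier based on the total.
; On BeginPlay it caches the GameInstance through a reference-getter message, and SetGameModeRef returns itself to callers.
; Each AddScroll increments the counter, prints the tally and runs SetTrophyType, which writes one of three threshold-based tiers to the GameInstance's Trophies.
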(event `self.ReceiveBeginPlay`
  ;[1 1 1] Begin Play
  (bind _gameinstance (message `/Game/Blueprints/Interfaces/INT_GameInstancee.SetGameInstanceRef` (`GameplayStatics.GetGameInstance`)))
  (set `self.Game Instance` _gameinstance))

(event `self.AddScroll`
  ;[1 1 1] Adding Scrolls when looted
  (bind _result (`/Engine/EditorBlueprintResources/StandardMacros.IncrementInt` (`self.ScrollCounter`))
    (:`  `
      (`KismetSystemLibrary.PrintString` (`KismetTextLibrary.Conv_TextToString` (`|FormatText` "You have looted {0} scrolls!" _result)))
      (`self.SetTrophyType`))))

(event `self.SetTrophyType`
  (bind _scrollcounter (`self.ScrollCounter`))
  (bind _game_instance (`self.Game Instance`))
  (if (<= _scrollcounter 2)
    (set `/Game/Blueprints/GI_DeathCollector.Trophies` "NewEnumerator0" _game_instance)
    (elif (and (> _scrollcounter 2) (<= _scrollcounter 5))
      (set `/Game/Blueprints/GI_DeathCollector.Trophies` "NewEnumerator1" _game_instance)
      (else
        (set `/Game/Blueprints/GI_DeathCollector.Trophies` "NewEnumerator2" _game_instance)))))

(fn `SetGameModeRef`
  (returns (GameMode :type "/Game/Blueprints/GM_DeathCollector Object Reference"))
  (return self))

(fn `UserConstructionScript`)